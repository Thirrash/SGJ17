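; Flying pillow actor that shows a key-prompt widget above a Paper2D flipbook sprite.
; Construction script randomly picks the black or white pillow flipbook.
; BeginPlay creates the PillowInput widget and plays a flying sound at the sprite's location.
; Tick projects a point just above the actor to screen space, moves the widget there and sets its text from KeyString.
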(event EventBeginPlay
  (bind _returnvalue (UserInterface|CreateWidget "/Game/PillowInput.PillowInput_C"))
  (UserInterface|Viewport|AddtoViewport _returnvalue 0)
  (Variables|Default|SetInputWidget _returnvalue)
  (Audio|PlaySoundatLocation "/Game/flying_pillow_Cue.flying_pillow_Cue" (Transformation|GetWorldLocation (Variables|Default|GetPaperFlipbook))))

(event EventTick
  (params (DeltaSeconds :type Float%20%28single-precision%29))
  (Class|UserWidget|SetPositioninViewport (stale EventBeginPlay _returnvalue) (.ScreenLocation (Class|PlayerController|ProjectWorldLocationtoScreen (Game|GetPlayerController 0) (+ (Transformation|GetActorLocation) "0, 0,20.000000") false)) true)
  (Variables|/Game/PillowInput.PillowInput_C|SetText (stale EventBeginPlay _returnvalue) (Variables|Default|GetKeyString)))

(fn ConstructionScript
  (if (Math|Conversions|ToBoolean(Integer) (Math|Random|RandomIntegerinRange 0 1))
    (Sprite|SetFlipbook (Variables|Default|GetPaperFlipbook) "/Game/Image/BlackPillow.BlackPillow")
    (else
      (Sprite|SetFlipbook (Variables|Default|GetPaperFlipbook) "/Game/Image/WhitePillow.WhitePillow"))))